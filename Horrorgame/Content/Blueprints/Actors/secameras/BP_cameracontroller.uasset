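; Security camera console actor that, when interacted with, lets the player view the level through its security cameras.
; BeginPlay gathers every BP_secCamera into an array, and Interact toggles viewing by moving input from the character to this actor and switching the view target.
; Space cycles through cameras with wraparound, while Return or Action restores character input and view.
; Entering and leaving also change the main HUD's visibility mode.
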(event Custom|leaeve
  (bind _returnvalue (Game|GetPlayerController 0))
  (Variables|Default|SetisViewingCAmera false)
  (Input|DisableInput _returnvalue)
  (Input|ResetIgnoreLookInput _returnvalue)
  (Widget|SetVisibility (Variables|/Game/GameBP/Level1/L1_Character.L1_Character_C|GetMainHudRef (.AsL1%20Character (Utilities|Casting|CastToL1_Character (Game|GetPlayerCharacter 0)))) "SelfHitTestInvisible")
  (Input|EnableInput (Game|GetPlayerCharacter 0) (Game|GetPlayerController 0))
  (Game|Player|SetViewTargetwithBlend (Game|GetPlayerController 0) (Game|GetPlayerCharacter 0) 0.0 "VTBlend_Linear" 0.0 false))

(event Collision|EventActorBeginOverlap
  (params (OtherActor :type Actor%20Object%20Reference)))

(event EventTick
  (params (DeltaSeconds :type Float%20%28single-precision%29)))

(event EventInteract
  (bind _returnvalue (Game|GetPlayerController 0))
  (if (Variables|Default|GetisViewingCAmera)
    (CallFunction|Leaeve)
    (else
      (Variables|Default|SetisViewingCAmera true)
      (Input|DisableInput (Game|GetPlayerCharacter 0) _returnvalue)
      (Input|SetIgnoreLookInput _returnvalue true)
      (Widget|SetVisibility (Variables|/Game/GameBP/Level1/L1_Character.L1_Character_C|GetMainHudRef (.AsL1%20Character (Utilities|Casting|CastToL1_Character (Game|GetPlayerCharacter 0)))) "Visible")
      (Input|EnableInput (Game|GetPlayerController 0))
      (CallFunction|Viewthroughcamera))))

(event EventBeginPlay
  (bind _outactors (Actor|GetAllActorsOfClass "/Game/Blueprints/Actors/secameras/BP_secCamera.BP_secCamera_C"))
  (Variables|Default|Setsecuritycameras _outactors))

(event Input|ActionEvents|InputActionReturn
  (params (Key :type Key%20Structure :default "None"))
  (:Pressed
    (CallFunction|Leaeve)))

(event Input|ActionEvents|InputActionAction
  (params (Key :type Key%20Structure :default "None"))
  (:Pressed
    (CallFunction|Leaeve)))

(event Input|KeyboardEvents|SpaceBar
  (params (Key :type Key%20Structure :default "None"))
  (:Pressed
    (Variables|Default|Setnumbercamera (select (> (+ (Variables|Default|Getnumbercamera) 1) (- (Utilities|Array|Length (Variables|Default|Getsecuritycameras)) 1)) 0 (+ (Variables|Default|Getnumbercamera) 1)))
    (CallFunction|Viewthroughcamera)))

(fn ConstructionScript)

(fn Viewthroughcamera
  (Game|Player|SetViewTargetwithBlend (Game|GetPlayerController 0) (Utilities|Array|Get(acopy) (Variables|Default|Getsecuritycameras) (Variables|Default|Getnumbercamera)) 0.0 "VTBlend_Linear" 0.0 false)
  (return))