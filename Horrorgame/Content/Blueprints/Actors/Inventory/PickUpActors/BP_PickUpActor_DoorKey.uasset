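; BP_PickUpActor_DoorKey is a door key pickup actor that reacts when the player character overlaps its static mesh.
; The overlap casts the other actor to L1_Character and increments that character's Pickup2 counter.
; It then compares the counter, converted to a boolean, with NewVar0, but both branches pause the game.
; The actor does not destroy or hide itself, and its BeginPlay and Tick events are disabled.
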(event OnComponentBeginOverlap(StaticMesh)
  (params (OverlappedComponent :type Primitive%20Component%20Object%20Reference) (OtherActor :type Actor%20Object%20Reference) (OtherComp :type Primitive%20Component%20Object%20Reference) (OtherBodyIndex :type Integer) (bFromSweep :type Boolean) (SweepResult :type Hit%20Result%20Structure%20%28by%20ref%29))
  (bind _asl1_character (Utilities|Casting|CastToL1_Character OtherActor))
  (Variables|/Game/GameBP/Level1/L1_Character.L1_Character_C|Setpickup2 _asl1_character (+ (Variables|/Game/GameBP/Level1/L1_Character.L1_Character_C|Getpickup2 _asl1_character) 1))
  (if (Math|Boolean|Equal(Boolean) (Math|Conversions|ToBoolean(Integer) (Variables|/Game/GameBP/Level1/L1_Character.L1_Character_C|Getpickup2 _asl1_character)) (Math|Conversions|ToBoolean(Integer) (Variables|Default|GetNewVar_0)))
    (Game|SetGamePaused true)
    (else
      (Game|SetGamePaused true))))

(event EventBeginPlay
  (|CallParentFunction) ; This node is disabled and will not be called.\nDrag off pins to build functionality.
)

(event EventTick
  (params (DeltaSeconds :type Float%20%28single-precision%29))
  (|CallParentFunction DeltaSeconds) ; This node is disabled and will not be called.\nDrag off pins to build functionality.
)

(fn ConstructionScript
  (|CallParentFunction))